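; Game HUD Blueprint that owns the on-screen crosshair widget and switches its focused state.
; On BeginPlay it creates WBP_Crosshair_UI, stores the reference and adds it to the viewport.
; Crosshair_FocusON and Crosshair_FocusOFF events call SetFocused on that widget.
; If the widget is invalid, either event recreates it instead, without applying the requested focus state.
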(event `self.ReceiveBeginPlay`
  (`self.InitCrosshairHUD`))

(event `InitCrosshairHUD`
  ;[1 1 1] Init Crosshair HUD
  (bind _returnvalue (`|CreateWidget` "/Game/Yuri/Blueprints/UI/WBP_Crosshair_UI.WBP_Crosshair_UI_C"))
  (bind _output_get (set `self.CrosshairHUD_` _returnvalue))
  (`UserWidget.AddToViewport` _output_get 0))

(event `Crosshair_FocusON`
  (bind _crosshairhud_ (`self.CrosshairHUD_`))
  ;[1 1 1] Toggle crosshair
  (`/Engine/EditorBlueprintResources/StandardMacros.IsValid` _crosshairhud_
    (:`Is Valid`
      (`/Game/Yuri/Blueprints/UI/WBP_Crosshair_UI.SetFocused` _crosshairhud_ true))
    (:`Is Not Valid`
      (`self.InitCrosshairHUD`))))

(event `Crosshair_FocusOFF`
  (bind _crosshairhud_ (`self.CrosshairHUD_`))
  ;[1 1 1] Toggle crosshair
  (`/Engine/EditorBlueprintResources/StandardMacros.IsValid` _crosshairhud_
    (:`Is Valid`
      (`/Game/Yuri/Blueprints/UI/WBP_Crosshair_UI.SetFocused` _crosshairhud_ false))
    (:`Is Not Valid`
      (`self.InitCrosshairHUD`))))

(fn `UserConstructionScript`)