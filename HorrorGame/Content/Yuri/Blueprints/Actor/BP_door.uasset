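; BP_door is an interactable door actor that toggles between open and closed on its Interact event.
; Open plays a locked sound if Locked is set; otherwise it plays the opening sound, slowly swings the Door component with MoveComponentTo and sets IsOpen.
; Close plays its sound, returns the door to zero rotation much faster and clears IsOpen.
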(event `/Game/Yuri/Interface/BPI_Interactable.Interact`
  ;[1 1 1] Interact
  (if (`self.IsOpen`)
    (`/Game/Yuri/Interface/BPI_Door.Close`)
    (else
      (`/Game/Yuri/Interface/BPI_Door.Open`))))

(event `/Game/Yuri/Interface/BPI_Door.Open`
  ;[1 1 1] Open Door
  (if (`self.Locked`)
    (`AudioComponent.Play` (`self.Doorlocked`) 0.0)
    (else
      (`AudioComponent.Play` (`self.Dooropen`) 0.0)
      (`KismetSystemLibrary.MoveComponentTo` (`self.Door`) (-100.0 0.0 0.0) (struct :`Yaw` 90.0) false false 6.3)
      (set `self.IsOpen` true))))

(event `/Game/Yuri/Interface/BPI_Door.Close`
  ;[1 1 1] Close Door
  (`AudioComponent.Play` (`self.Doorclose`) 0.0)
  (`KismetSystemLibrary.MoveComponentTo` (`self.Door`) (-100.0 0.0 0.0) (struct) false false 1.2)
  (set `self.IsOpen` false))

(fn `UserConstructionScript`)