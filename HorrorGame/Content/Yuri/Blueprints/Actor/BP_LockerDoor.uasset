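; BP_LockerDoor is an interactable locker door that players can swing open and closed.
; Interact toggles between the Open and Close events based on IsOpen, and does nothing while Locked.
; Each event rotates the Door component with a short MoveComponentTo, plays its own sound and updates IsOpen.
; Open also checks Locked itself, while Close runs regardless of the lock.
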(event `/Game/Yuri/Interface/BPI_Interactable.Interact`
  ;[1 1 1] Interact
  (if (`self.Locked`)
    _
    (elif (`self.IsOpen`)
      (`/Game/Yuri/Interface/BPI_Door.Close`)
      (else
        (`/Game/Yuri/Interface/BPI_Door.Open`)))))

(event `/Game/Yuri/Interface/BPI_Door.Open`
  ;[1 1 1] Open Door
  (if (not (`self.Locked`))
    (`AudioComponent.Play` (`self.MS_lockerdooropen`) 0.0)
    (`KismetSystemLibrary.MoveComponentTo` (`self.Door`) (0.0 0.0 0.0) (struct :`Yaw` -90.0) false false 0.4)
    (set `self.IsOpen` true)))

(event `/Game/Yuri/Interface/BPI_Door.Close`
  ;[1 1 1] Close Door
  (`KismetSystemLibrary.MoveComponentTo` (`self.Door`) (0.0 0.0 0.0) (struct) false false 0.4)
  (set `self.IsOpen` false)
  (`AudioComponent.Play` (`self.MS_lockerdoorclose`) 0.0))

(fn `UserConstructionScript`)